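; BP_TargettingNet is a combat targeting helper that gathers the targetable pawns overlapping its sphere.
; GetTargetsInRange filters overlaps through the IsCombatTargettableMessage interface call and separates out those absent from the ACTargetSystem's RecentlyTargetted list.
; It returns these fresh targets first; when none remain, it clears that history and returns all targets in range, allowing target cycling.
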(fn `GetTargetsInRange`
  (returns (Targets :type "Array of Actor Object Reference"))
  (locals (TargetsInRange :type "Array of Actor Object Reference") (FreshTargetInRange :type "Array of Actor Object Reference"))
  (bind _freshtargetinrange (`local.FreshTargetInRange`))
  (for _array_element (`PrimitiveComponent.GetOverlappingActors` (`self.Sphere`) "/Script/Engine.Pawn")
    (bind _istargettable (message `/Game/CombatSystem/Interfaces/BPI_Target.IsCombatTargettable` _array_element))
    (if _istargettable
      (`KismetArrayLibrary.Array_AddUnique` (`local.TargetsInRange`) _array_element)
      (if (not (`KismetArrayLibrary.Array_Contains` (`/Game/CombatSystem/Components/AC_TargetSystem.RecentlyTargetted` (`self.AC_TargetSystem`)) _array_element))
        (`KismetArrayLibrary.Array_AddUnique` (`local.FreshTargetInRange`) _array_element))))
  (if (`KismetArrayLibrary.Array_IsEmpty` _freshtargetinrange)
    (`KismetArrayLibrary.Array_Clear` (`/Game/CombatSystem/Components/AC_TargetSystem.RecentlyTargetted` (`self.AC_TargetSystem`)))
    (return (`local.TargetsInRange`))
    (else
      (return _freshtargetinrange))))

(fn `UserConstructionScript`)