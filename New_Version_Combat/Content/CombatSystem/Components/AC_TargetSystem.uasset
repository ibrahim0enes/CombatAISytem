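; Lock-on targeting component that, on Tab or TriggerTargetting, selects a nearby enemy or other actor to face.
; A spawned BP_TargettingNet supplies candidates; the closest becomes CurrentTarget, gets an attached BP_Targetter marker, and new/clear events notify listeners.
; Tick smoothly interpolates owner and first player controller yaw toward the target.
; A retriggerable delay resets the RecentlyTargetted list to the current target, though selection here never reads it.
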(event `self.ReceiveBeginPlay`
  (bind _asbp_third_person_character (cast `/Game/ThirdPerson/Blueprints/BP_ThirdPersonCharacter` (`self.GetOwner`)))
  (set `self.As BP Third Person Character` _asbp_third_person_character))

(event `Trigger Targetting`
  (bind _recentlytargetted (`self.RecentlyTargetted`))
  (bind _returnvalue (`|SpawnActorFromClass` "/Game/CombatSystem/Actor/BP_TargettingNet.BP_TargettingNet_C" (`Actor.GetTransform` (`self.GetOwner`)) "AlwaysSpawn" "MultiplyWithRoot" null null :!label _label))
  (bind _targets (`/Game/CombatSystem/Actor/BP_TargettingNet.GetTargetsInRange` _returnvalue))
  (bind _closest (`self.GetClosestActor` _targets))
  (`self.CleanActor`)
  (`self.TargetActor` _closest)
  (`KismetSystemLibrary.RetriggerableDelay` 3.0)
  (`KismetArrayLibrary.Array_Clear` _recentlytargetted)
  (bind _currenttarget (`self.CurrentTarget`)
    (:`then`
      (`KismetArrayLibrary.Array_AddUnique` _recentlytargetted _currenttarget))
    (:`else`)))

(event `Key|Tab`
  (params (Key :type "Key Structure"))
  (:`Pressed`
    (goto _label)))

(event `self.ReceiveTick`
  (params (DeltaSeconds :type "Float (single-precision)"))
  (bind (_returnvalue_roll _returnvalue_pitch) (`KismetMathLibrary.BreakRotator` (`Actor.K2_GetActorRotation` (`self.GetOwner`))))
  (bind (_returnvalue_roll_2 _returnvalue_pitch_2) (`KismetMathLibrary.BreakRotator` (`Controller.GetControlRotation` (`GameplayStatics.GetPlayerController` 0))))
  ; Set Rotation to Target Actor
  (bind _currenttarget (`self.CurrentTarget`)
    (:`then`
      (bind (_returnvalue_x _returnvalue_y _returnvalue_z) (`KismetMathLibrary.BreakVector` (`Actor.K2_GetActorLocation` _currenttarget)))
      (bind (_returnvalue_roll_3 _returnvalue_pitch_3 _returnvalue_yaw) (`KismetMathLibrary.BreakRotator` (`KismetMathLibrary.FindLookAtRotation` (`Actor.K2_GetActorLocation` (`self.GetOwner`)) (`KismetMathLibrary.MakeVector` _returnvalue_x _returnvalue_y (- _returnvalue_z 44.0)))))
      (`Actor.K2_SetActorRotation` (`self.GetOwner`) (`KismetMathLibrary.RInterpTo` (`Actor.K2_GetActorRotation` (`self.GetOwner`)) (`KismetMathLibrary.MakeRotator` _returnvalue_roll _returnvalue_pitch _returnvalue_yaw) (`GameplayStatics.GetWorldDeltaSeconds`) 4.0) false)
      (`Controller.SetControlRotation` (`GameplayStatics.GetPlayerController` 0) (`KismetMathLibrary.RInterpTo` (`Controller.GetControlRotation` (`GameplayStatics.GetPlayerController` 0)) (`KismetMathLibrary.MakeRotator` _returnvalue_roll_2 _returnvalue_pitch_2 _returnvalue_yaw) (`GameplayStatics.GetWorldDeltaSeconds`) 3.0)))
    (:`else`)))

(fn `CleanActor`
  (set `self.CurrentTarget` null)
  (bind _targetter (`self.Targetter`)
    (:`then`
      (`Actor.K2_DestroyActor` _targetter)
      (`self.OnClearTarget`))
    (:`else`)))

(fn `GetClosestActor`
  (params (Actor :type "Array of Actor Object Reference"))
  (returns (Closest :type "Actor Object Reference") (Distance :type "Float (double-precision)"))
  (locals (ClosestActor :type "Actor Object Reference") (ClosestDistance :type "Float (double-precision)" :default 2000.0))
  (for _array_element Actor
    (bind _returnvalue (`Actor.GetDistanceTo` _array_element (`self.GetOwner`)))
    (if (< _returnvalue (`local.ClosestDistance`))
      (set `local.ClosestDistance` _returnvalue)
      (set `local.ClosestActor` _array_element)
      (else
        (`self.CleanActor`))))
  (return (`local.ClosestActor`) (`local.ClosestDistance`)))

(fn `IsCombatTargettable`
  (returns (IsTargettable :type Boolean))
  (return false))

(fn `TargetActor`
  (params (Actor :type "Actor Object Reference"))
  (`/Engine/EditorBlueprintResources/StandardMacros.IsValid` Actor
    (:`Is Valid`
      (bind _output_get (set `self.CurrentTarget` Actor))
      (`KismetArrayLibrary.Array_AddUnique` (`self.RecentlyTargetted`) _output_get)
      (bind _returnvalue (`|SpawnActorFromClass` "/Game/CombatSystem/Actor/BP_Targetter.BP_Targetter_C" (`Actor.GetTransform` _output_get) "AlwaysSpawn" "MultiplyWithRoot" null null))
      (bind _output_get_2 (set `self.Targetter` _returnvalue))
      (`Actor.K2_AttachToActor` _output_get_2 (`self.CurrentTarget`) "None" "KeepWorld" "KeepWorld" "KeepWorld" true)
      (`self.OnNewTarget` (`self.CurrentTarget`)))))